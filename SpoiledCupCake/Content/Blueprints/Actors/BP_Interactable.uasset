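; BP_Interactable is an actor that toggles between closed and open when Interact fires, moving its Up component vertically.
; Two timelines lerp Up's relative location from its current position toward a raised offset or back to the origin, flipping the Closed flag on finish.
; A DoOnce blocks re-triggering until the move ends.
; Overlapping InteractTrigger with BP_CupCake shows a Text prompt, which hides when the overlap ends.
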(event OnComponentBeginOverlap(InteractTrigger)
  (params (OverlappedComponent :type Primitive%20Component%20Object%20Reference) (OtherActor :type Actor%20Object%20Reference) (OtherComp :type Primitive%20Component%20Object%20Reference) (OtherBodyIndex :type Integer) (bFromSweep :type Boolean) (SweepResult :type Hit%20Result%20Structure%20%28by%20ref%29))
  (Utilities|Casting|CastToBP_CupCake OtherActor)
  (Development|SetHiddeninGame (Variables|Default|GetText) false false))

(event OnComponentEndOverlap(InteractTrigger)
  (params (OverlappedComponent :type Primitive%20Component%20Object%20Reference) (OtherActor :type Actor%20Object%20Reference) (OtherComp :type Primitive%20Component%20Object%20Reference) (OtherBodyIndex :type Integer))
  (Utilities|Casting|CastToBP_CupCake OtherActor)
  (Development|SetHiddeninGame (Variables|Default|GetText) true false))

(event EventBeginPlay)

(event Collision|EventActorBeginOverlap
  (params (OtherActor :type Actor%20Object%20Reference)))

(event EventTick
  (params (DeltaSeconds :type Float%20%28single-precision%29)))

(event EventInteract
  (Utilities|FlowControl|DoOnce false :!label _label
    (:Completed
      (if (Variables|Default|GetClosed)
        (bind _movespeed (Timeline|Move%20Up PlayFromStart)
          (:Update
            (Transformation|SetRelativeLocation (Variables|Default|GetUp) (Math|Vector|Lerp(Vector) (.location (Transformation|GetRelativeTransform (Variables|Default|GetUp))) "0, 0,90.000000" _movespeed) false false))
          (:Finished
            (Variables|Default|SetClosed false)
            (goto _label Reset)))
        (else
          (bind _movement (Timeline|Reset PlayFromStart)
            (:Update
              (Transformation|SetRelativeLocation (Variables|Default|GetUp) (Math|Vector|Lerp(Vector) (.location (Transformation|GetRelativeTransform (Variables|Default|GetUp))) "0, 0, 0" _movement) false false))
            (:Finished
              (Variables|Default|SetClosed true)
              (goto _label Reset))))))))

(fn ConstructionScript)