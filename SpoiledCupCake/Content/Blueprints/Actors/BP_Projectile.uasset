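; BP_Projectile is an attack actor that knocks back or kills a BP_CupCake character on contact.
; Its SphereTrigger overlap checks the cupcake's Blocked flag: a blocked attack applies a small fixed-direction push and destroys the projectile.
; An unblocked attack launches the cupcake upward, prints a death message, then disables its movement and destroys the projectile after a delay.
; A component hit against a cupcake also destroys the projectile.
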(event OnComponentBeginOverlap(SphereTrigger)
  (params (OverlappedComponent :type Primitive%20Component%20Object%20Reference) (OtherActor :type Actor%20Object%20Reference) (OtherComp :type Primitive%20Component%20Object%20Reference) (OtherBodyIndex :type Integer) (bFromSweep :type Boolean) (SweepResult :type Hit%20Result%20Structure%20%28by%20ref%29))
  (bind _asbp_cup_cake (Utilities|Casting|CastToBP_CupCake OtherActor))
  (Variables|Default|SetPlayerRef _asbp_cup_cake)
  (if (Variables|/Game/Assets/PaperZD/BP_CupCake.BP_CupCake_C|GetBlocked (Variables|Default|GetPlayerRef))
    (Development|PrintString "Attack has been blocked")
    (Physics|AddImpulse (Variables|/Script/Engine.Character|GetCharacterMovement (Variables|Default|GetPlayerRef)) "100.000000,0.000000,50.000000" true)
    (Actor|DestroyActor)
    (else
      (Development|PrintString "Player died")
      (Physics|AddImpulse (Variables|/Script/Engine.Character|GetCharacterMovement (Variables|Default|GetPlayerRef)) "0.000000,0.000000,500.000000" true)
      (Utilities|FlowControl|Delay 2.0)
      (Pawn|Components|CharacterMovement|DisableMovement (Variables|/Script/Engine.Character|GetCharacterMovement (Variables|Default|GetPlayerRef)))
      (Actor|DestroyActor))))

(event OnComponentHit(SphereTrigger)
  (params (HitComponent :type Primitive%20Component%20Object%20Reference) (OtherActor :type Actor%20Object%20Reference) (OtherComp :type Primitive%20Component%20Object%20Reference) (NormalImpulse :type Vector :default "0, 0, 0") (Hit :type Hit%20Result%20Structure%20%28by%20ref%29))
  (Utilities|Casting|CastToBP_CupCake OtherActor)
  (Actor|DestroyActor self))

(event EventBeginPlay)

(event Collision|EventActorBeginOverlap
  (params (OtherActor :type Actor%20Object%20Reference)))

(event EventTick
  (params (DeltaSeconds :type Float%20%28single-precision%29)))

(fn ConstructionScript)